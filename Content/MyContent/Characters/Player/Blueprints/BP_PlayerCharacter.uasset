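; Player character Blueprint that casts the A_Gale ability on Cast input through CastAbility; the BP_CastAbility event is empty.
; Two helper macros build an ability context and activate it on AbilityComponent, with the passive variant also setting a non-zero stack count and resetting duration.
; IsnearCharacter sphere-traces around CentralComponent once an ability has run over a second, returning the hit actor.
; No shown graph calls these helpers.
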(event EventBeginPlay)

(event Collision|EventActorBeginOverlap
  (params (OtherActor :type Actor%20Object%20Reference)))

(event EventTick
  (params (DeltaSeconds :type Float%20%28single-precision%29)))

(event Input|ActionEvents|InputActionCast
  (params (Key :type Key%20Structure)))

(event Custom|BP_CastAbility
  (params (Ability :type Abl%20Ability%20Object%20Reference) (Instigator :type Actor%20Object%20Reference) (NewStackCount :type Integer)))

(event Input|ActionEvents|InputActionCast
  (params (Key :type Key%20Structure :default "None"))
  (:Pressed
    (Class|BaseCharacter|CastAbility (Class|AblAbilityBlueprintLibrary|GetAbilityObjectfromClass "/Game/MyContent/Abilities/Gale/A_Gale.A_Gale_C") self)))

(fn ConstructionScript)

(fn IsnearCharacter
  (params (Ability :type Abl%20Ability%20Object%20Reference))
  (bind _centralcomponent (Variables|Default|GetCentralComponent))
  (bind _returnvalue (Transformation|GetWorldLocation _centralcomponent))
  (if (> (Class|AblAbilityComponent|GetAbilityCurrentTime (Variables|Default|GetAbilityComponent) Ability) 1.0)
    (bind (_outhit _returnvalue_2) (Collision|SphereTraceByChannel _returnvalue _returnvalue 125.0 "TraceTypeQuery3" false 0 "ForOneFrame"))
    (if _returnvalue_2
      (return (.hitactor _outhit)))))