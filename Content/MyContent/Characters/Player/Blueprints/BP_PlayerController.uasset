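; BP_PlayerController is the player controller that turns input into movement, camera look and jumping for BP_PlayerCharacter.
; Move axes cast the controlled pawn to BP_PlayerCharacter and add movement along its forward and right vectors.
; Look axes feed pitch and yaw input directly on the controller.
; The Jump action starts jumping on press and stops it on release through the same pawn cast.
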(event EventBeginPlay)

(event EventTick
  (params (DeltaSeconds :type Float%20%28single-precision%29)))

(event Input|ActionEvents|InputActionJump
  (params (Key :type Key%20Structure))
  (bind _returnvalue (Pawn|GetControlledPawn))
  (:Pressed
    (bind _asbp_player_character (Utilities|Casting|CastToBP_PlayerCharacter _returnvalue))
    (Character|Jump _asbp_player_character))
  (:Released
    (bind _asbp_player_character_2 (Utilities|Casting|CastToBP_PlayerCharacter _returnvalue))
    (Character|StopJumping _asbp_player_character_2)))

(event Input|AxisEvents|InputAxisMoveForward
  (params (AxisValue :type Float%20%28single-precision%29))
  (bind _asbp_player_character (Utilities|Casting|CastToBP_PlayerCharacter (Pawn|GetControlledPawn)))
  (Pawn|Input|AddMovementInput _asbp_player_character (Transformation|GetActorForwardVector _asbp_player_character) AxisValue false))

(event Input|AxisEvents|InputAxisMoveRight
  (params (AxisValue :type Float%20%28single-precision%29))
  (bind _asbp_player_character (Utilities|Casting|CastToBP_PlayerCharacter (Pawn|GetControlledPawn)))
  (Pawn|Input|AddMovementInput _asbp_player_character (Transformation|GetActorRightVector _asbp_player_character) AxisValue false))

(event Input|AxisEvents|InputAxisLookUp
  (params (AxisValue :type Float%20%28single-precision%29))
  (Class|PlayerController|AddPitchInput AxisValue))

(event Input|AxisEvents|InputAxisLookRight
  (params (AxisValue :type Float%20%28single-precision%29))
  (Class|PlayerController|AddYawInput AxisValue))

(fn ConstructionScript)